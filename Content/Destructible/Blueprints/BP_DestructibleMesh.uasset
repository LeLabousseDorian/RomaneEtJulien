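; BP_DestructibleMesh is a destructible prop that awards score to the player when it fractures.
; On fracture, the destructible component applies a constant-falloff radial force at its own location to push the pieces.
; The first fracture that finds a BP_MyController as player controller 0 adds Score to it and sets ScoreGiven to prevent repeat awards.
; IsDestroyed always returns false, regardless of fracture state.
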(event OnComponentFracture(DestructibleComponent)
  (params (HitPoint :type Vector%20%28by%20ref%29 :default "0, 0, 0") (HitDirection :type Vector%20%28by%20ref%29 :default "0, 0, 0"))
  (Physics|AddRadialForce (Variables|Default|GetDestructibleComponent) (Transformation|GetWorldLocation (Variables|Default|GetDestructibleComponent)) 1e+02 3e+05 "RIF_Constant" false)
  (if (not (Variables|Default|GetScoreGiven))
    (bind _asbp_my_controller (Utilities|Casting|CastToBP_MyController (Game|GetPlayerController 0)))
    (Default|AddScore _asbp_my_controller (Variables|Default|GetScore))
    (Variables|Default|SetScoreGiven true)))

(fn ConstructionScript)

(fn IsDestroyed
  (return false))